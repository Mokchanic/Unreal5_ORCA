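; BP_Pedestrian is a walking pedestrian that records its trajectory to a per-ID CSV file.
; Reset moves it to a random Spawner transform, randomizes height scale and walk speed, then AI-moves it straight ahead by MoveDistance.
; While moving, Tick smoothly turns it toward its velocity and, once the spawner finishes summoning, logs X, Y and yaw.
; A 15-second Delay in Tick triggers a one-time save of that log.
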(event `SetID`
  (params (PedID :type Integer))
  (set `self.Ped ID` PedID))

(event `self.ReceiveBeginPlay`
  (bind _outactors (`GameplayStatics.GetAllActorsOfClass` "/Game/MyContent/BluePrints/Pedestrian/BP_Pedestrian.BP_Pedestrian_C"))
  (set `self.Pedestrian` _outactors)
  (`KismetArrayLibrary.Array_Clear` (`self.PedPoseList`)))

(event `Reset`
  (`self.K2_SetActorTransform` (`/Game/MyContent/BluePrints/BP_Spawner.MakeRandomSpawnTransform` (`self.Spawner`)) false true)
  (`self.SetScale`)
  (`self.SetSpeed`)
  (bind _output_get (set `self.Target` (+ (* (`KismetMathLibrary.GetForwardVector` (`self.K2_GetActorRotation`)) (`self.MoveDistance`)) (`self.K2_GetActorLocation`))))
  (`|AIMoveTo` self _output_get null 50.0
    (:`OnSuccess`
      _)
    (:`OnFail`
      _))
  (`/Game/MyContent/BluePrints/BP_Spawner.PathEnd` (`self.Spawner`) null))

(event `self.ReceiveTick`
  (params (DeltaSeconds :type "Float (single-precision)"))
  (bind _returnvalue (`self.GetTransform`))
  (if (< 5.0 (`KismetMathLibrary.VSize` (`self.GetVelocity`)))
    (`self.CalSetActorRotate`)
    (bind _returnvalue_2 (`GameplayStatics.GetActorOfClass` "/Game/MyContent/BluePrints/BP_Spawner.BP_Spawner_C"))
    (if (`/Game/MyContent/BluePrints/BP_Spawner.SummonsComplete` _returnvalue_2)
      (`KismetArrayLibrary.Array_Add` (`self.PedPoseList`) (`KismetStringLibrary.Concat_StrStr` (`KismetStringLibrary.Conv_DoubleToString` (.x (.location _returnvalue))) "," (`KismetStringLibrary.Conv_DoubleToString` (.y (.location _returnvalue))) "," (`KismetStringLibrary.Conv_DoubleToString` (.yaw (.rotation _returnvalue)))))
      (`KismetSystemLibrary.Delay` 15.0)
      (if (not (`self.MakeData`))
        (`RWTxt.FileSaveString` (`KismetStringLibrary.JoinStringArray` (`self.PedPoseList`) ",") (`KismetStringLibrary.Concat_StrStr` (`KismetStringLibrary.Conv_IntToString` (`self.Ped ID`)) "complete.csv"))
        (set `self.MakeData` true)
        (`KismetSystemLibrary.PrintString` "MakeCSV!" true true (struct :`R` 1.0 :`B` 0.009271 :`A` 1.0) 30.0)))))

(fn `AppendLocationArray`
  (bind (_returnvalue_x _returnvalue_y) (`KismetMathLibrary.BreakVector` (`self.K2_GetActorLocation`)))
  (`KismetArrayLibrary.Array_Append` (`self.PedPoseList`) (`|MakeArray` (`KismetStringLibrary.Conv_DoubleToString` _returnvalue_x) (`KismetStringLibrary.Conv_DoubleToString` _returnvalue_y))))

(fn `CalSetActorRotate`
  (bind (_returnvalue_roll _returnvalue_pitch _returnvalue_yaw) (`KismetMathLibrary.BreakRotator` (`KismetMathLibrary.RInterpTo` (`self.K2_GetActorRotation`) (`KismetMathLibrary.FindLookAtRotation` (`KismetMathLibrary.MakeVector` 0.0) (`self.GetVelocity`)) (`GameplayStatics.GetWorldDeltaSeconds`) 8.0)))
  (`self.K2_SetActorRotation` (`KismetMathLibrary.MakeRotator` 0.0 0.0 _returnvalue_yaw) true))

(fn `DrawArrow`
  (`KismetSystemLibrary.DrawDebugArrow` (`self.K2_GetActorLocation`) (`self.Target`) 15.0 (struct :`R` 1.0 :`G` 0.016606 :`A` 1.0) 0.0 10.0))

(fn `SetRandomSpeed`
  (set `CharacterMovementComponent.MaxWalkSpeed` (`KismetMathLibrary.RandomFloatInRange` (`KismetMathLibrary.RandomFloatInRange` 10.0 150.0) (`KismetMathLibrary.RandomFloatInRange` 151.0 300.0)) (`self.CharacterMovement`)))

(fn `SetScale`
  (bind _output_get (set `self.Height` (/ (`KismetMathLibrary.RandomFloatInRange` 150.0 190.0) 180.0)))
  (`self.SetActorScale3D` (`KismetMathLibrary.MakeVector` _output_get _output_get _output_get)))

(fn `SetSpeed`
  (set `CharacterMovementComponent.MaxWalkSpeed` (`KismetMathLibrary.RandomFloatInRange` 90.0 300.0) (`self.CharacterMovement`)))

(fn `StartOverlap`
  (params (OtherActor1 :type "Actor Object Reference") (OtherActor2 :type "Object Object Reference") (OtherComp :type "PrimitiveComponent Object Reference"))
  (if (`self.bInitPed`)
    _
    (elif (not (== OtherActor2 self))
      (bind _asbp_pedestrian (cast `/Game/MyContent/BluePrints/Pedestrian/BP_Pedestrian` OtherActor1))
      (if (== (`Character.Mesh` _asbp_pedestrian) OtherComp)
        (`KismetSystemLibrary.PrintString` "overlap")))))

(fn `UserConstructionScript`)