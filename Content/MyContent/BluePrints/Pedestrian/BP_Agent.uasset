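; BP_Agent is an agent that optionally walks straight ahead via AI MoveTo while recording nearby pedestrians.
; Sixteen sphere components each count BP_Pedestrian capsule begin-overlaps and append the agent-relative X/Y offset to ListAxisPoints.
; Tick draws a debug arrow to the target and, through a ten-second Delay, calls MakeCav to append MainSphereOverlap's per-sphere count outputs to TotalCountPoint.
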(event `MakeCav`
  (`KismetArrayLibrary.Array_Append` (`self.TotalCountPoint`) (`|MakeArray` (`self.iCountSphere1-1`) (`self.iCountSphere1-2`) (`self.iCountSphere1-3`) (`self.iCountSphere1-4`) (`self.iCountSphere1-5`) (`self.iCountSphere1-6`) (`self.iCountSphere1-7`) (`self.iCountSphere1-8`) (`self.iCountSphere1-9`) (`self.iCountSphere1-10`) (`self.iCountSphere1-11`) (`self.iCountSphere1-12`) (`self.iCountSphere1-13`) (`self.iCountSphere1-13`) (`self.iCountSphere1-14`) (`self.iCountSphere1-15`) (`self.iCountSphere1-16`))))

(event `self.ReceiveBeginPlay`
  ;[1 1 1] Main
  (bind _returnvalue (`GameplayStatics.GetActorOfClass` "BP_Agent_C"))
  (set `self.Agent` _returnvalue)
  (if (`self.IsWaik`)
    (`KismetSystemLibrary.Delay` 0.0)
    (set `CharacterMovementComponent.MaxWalkSpeed` (`self.fAgentSpeed`) (`self.CharacterMovement`))
    (bind _output_get (`self.SetTarget`))
    (`|AIMoveTo` self _output_get null 50.0
      (:`OnSuccess`
        (`KismetSystemLibrary.PrintString` "Done!")))))

(event `self.ReceiveTick`
  (params (DeltaSeconds :type "Float (single-precision)"))
  ;[1 1 1] Main
  (`self.DrawArrow`)
  (`KismetSystemLibrary.Delay` 10.0)
  (`self.MakeCav`))

(event `self.Sphere1-1.OnComponentBeginOverlap`
  (params (OverlappedComponent :type "PrimitiveComponent Object Reference") (OtherActor :type "Actor Object Reference") (OtherComp :type "PrimitiveComponent Object Reference") (OtherBodyIndex :type Integer) (bFromSweep :type Boolean) (SweepResult :type "HitResult Structure (by ref)"))
  ;[1 1 1] MainSphere1
  (bind _asbp_pedestrian (cast `/Game/MyContent/BluePrints/Pedestrian/BP_Pedestrian` OtherActor))
  (bind _capsulecomponent (`Character.CapsuleComponent` _asbp_pedestrian))
  (if (== _capsulecomponent OtherComp)
    (`/Engine/EditorBlueprintResources/StandardMacros.IncrementInt` (`self.iCountSphere1-1`)
      (:`  `
        (bind (_returnvalue_x _returnvalue_y) (`KismetMathLibrary.BreakVector` (- (`self.K2_GetActorLocation`) (`SceneComponent.K2_GetComponentLocation` _capsulecomponent))))
        (`KismetArrayLibrary.Array_Append` (`self.ListAxisPoints`) (`|MakeArray` _returnvalue_x _returnvalue_y))))))

(event `self.Sphere1-9.OnComponentBeginOverlap`
  (params (OverlappedComponent :type "PrimitiveComponent Object Reference") (OtherActor :type "Actor Object Reference") (OtherComp :type "PrimitiveComponent Object Reference") (OtherBodyIndex :type Integer) (bFromSweep :type Boolean) (SweepResult :type "HitResult Structure (by ref)"))
  ;[1 1 1] MainSphere1
  (bind _asbp_pedestrian (cast `/Game/MyContent/BluePrints/Pedestrian/BP_Pedestrian` OtherActor))
  (bind _capsulecomponent (`Character.CapsuleComponent` _asbp_pedestrian))
  (if (== _capsulecomponent OtherComp)
    (`/Engine/EditorBlueprintResources/StandardMacros.IncrementInt` (`self.iCountSphere1-9`)
      (:`  `
        (bind (_returnvalue_x _returnvalue_y) (`KismetMathLibrary.BreakVector` (- (`self.K2_GetActorLocation`) (`SceneComponent.K2_GetComponentLocation` _capsulecomponent))))
        (`KismetArrayLibrary.Array_Append` (`self.ListAxisPoints`) (`|MakeArray` _returnvalue_x _returnvalue_y))))))

(event `self.Sphere1-2.OnComponentBeginOverlap`
  (params (OverlappedComponent :type "PrimitiveComponent Object Reference") (OtherActor :type "Actor Object Reference") (OtherComp :type "PrimitiveComponent Object Reference") (OtherBodyIndex :type Integer) (bFromSweep :type Boolean) (SweepResult :type "HitResult Structure (by ref)"))
  ;[1 1 1] MainSphere1
  (bind _asbp_pedestrian (cast `/Game/MyContent/BluePrints/Pedestrian/BP_Pedestrian` OtherActor))
  (bind _capsulecomponent (`Character.CapsuleComponent` _asbp_pedestrian))
  (if (== _capsulecomponent OtherComp)
    (`/Engine/EditorBlueprintResources/StandardMacros.IncrementInt` (`self.iCountSphere1-2`)
      (:`  `
        (bind (_returnvalue_x _returnvalue_y) (`KismetMathLibrary.BreakVector` (- (`self.K2_GetActorLocation`) (`SceneComponent.K2_GetComponentLocation` _capsulecomponent))))
        (`KismetArrayLibrary.Array_Append` (`self.ListAxisPoints`) (`|MakeArray` _returnvalue_x _returnvalue_y))))))

(event `self.Sphere1-10.OnComponentBeginOverlap`
  (params (OverlappedComponent :type "PrimitiveComponent Object Reference") (OtherActor :type "Actor Object Reference") (OtherComp :type "PrimitiveComponent Object Reference") (OtherBodyIndex :type Integer) (bFromSweep :type Boolean) (SweepResult :type "HitResult Structure (by ref)"))
  ;[1 1 1] MainSphere1
  (bind _asbp_pedestrian (cast `/Game/MyContent/BluePrints/Pedestrian/BP_Pedestrian` OtherActor))
  (bind _capsulecomponent (`Character.CapsuleComponent` _asbp_pedestrian))
  (if (== _capsulecomponent OtherComp)
    (`/Engine/EditorBlueprintResources/StandardMacros.IncrementInt` (`self.iCountSphere1-10`)
      (:`  `
        (bind (_returnvalue_x _returnvalue_y) (`KismetMathLibrary.BreakVector` (- (`self.K2_GetActorLocation`) (`SceneComponent.K2_GetComponentLocation` _capsulecomponent))))
        (`KismetArrayLibrary.Array_Append` (`self.ListAxisPoints`) (`|MakeArray` _returnvalue_x _returnvalue_y))))))

(event `self.Sphere1-3.OnComponentBeginOverlap`
  (params (OverlappedComponent :type "PrimitiveComponent Object Reference") (OtherActor :type "Actor Object Reference") (OtherComp :type "PrimitiveComponent Object Reference") (OtherBodyIndex :type Integer) (bFromSweep :type Boolean) (SweepResult :type "HitResult Structure (by ref)"))
  ;[1 1 1] MainSphere1
  (bind _asbp_pedestrian (cast `/Game/MyContent/BluePrints/Pedestrian/BP_Pedestrian` OtherActor))
  (bind _capsulecomponent (`Character.CapsuleComponent` _asbp_pedestrian))
  (if (== _capsulecomponent OtherComp)
    (`/Engine/EditorBlueprintResources/StandardMacros.IncrementInt` (`self.iCountSphere1-3`)
      (:`  `
        (bind (_returnvalue_x _returnvalue_y) (`KismetMathLibrary.BreakVector` (- (`self.K2_GetActorLocation`) (`SceneComponent.K2_GetComponentLocation` _capsulecomponent))))
        (`KismetArrayLibrary.Array_Append` (`self.ListAxisPoints`) (`|MakeArray` _returnvalue_x _returnvalue_y))))))

(event `self.Sphere1-11.OnComponentBeginOverlap`
  (params (OverlappedComponent :type "PrimitiveComponent Object Reference") (OtherActor :type "Actor Object Reference") (OtherComp :type "PrimitiveComponent Object Reference") (OtherBodyIndex :type Integer) (bFromSweep :type Boolean) (SweepResult :type "HitResult Structure (by ref)"))
  ;[1 1 1] MainSphere1
  (bind _asbp_pedestrian (cast `/Game/MyContent/BluePrints/Pedestrian/BP_Pedestrian` OtherActor))
  (bind _capsulecomponent (`Character.CapsuleComponent` _asbp_pedestrian))
  (if (== _capsulecomponent OtherComp)
    (`/Engine/EditorBlueprintResources/StandardMacros.IncrementInt` (`self.iCountSphere1-11`)
      (:`  `
        (bind (_returnvalue_x _returnvalue_y) (`KismetMathLibrary.BreakVector` (- (`self.K2_GetActorLocation`) (`SceneComponent.K2_GetComponentLocation` _capsulecomponent))))
        (`KismetArrayLibrary.Array_Append` (`self.ListAxisPoints`) (`|MakeArray` _returnvalue_x _returnvalue_y))))))

(event `self.Sphere1-4.OnComponentBeginOverlap`
  (params (OverlappedComponent :type "PrimitiveComponent Object Reference") (OtherActor :type "Actor Object Reference") (OtherComp :type "PrimitiveComponent Object Reference") (OtherBodyIndex :type Integer) (bFromSweep :type Boolean) (SweepResult :type "HitResult Structure (by ref)"))
  ;[1 1 1] MainSphere1
  (bind _asbp_pedestrian (cast `/Game/MyContent/BluePrints/Pedestrian/BP_Pedestrian` OtherActor))
  (bind _capsulecomponent (`Character.CapsuleComponent` _asbp_pedestrian))
  (if (== _capsulecomponent OtherComp)
    (`/Engine/EditorBlueprintResources/StandardMacros.IncrementInt` (`self.iCountSphere1-4`)
      (:`  `
        (bind (_returnvalue_x _returnvalue_y) (`KismetMathLibrary.BreakVector` (- (`self.K2_GetActorLocation`) (`SceneComponent.K2_GetComponentLocation` _capsulecomponent))))
        (`KismetArrayLibrary.Array_Append` (`self.ListAxisPoints`) (`|MakeArray` _returnvalue_x _returnvalue_y))))))

(event `self.Sphere1-12.OnComponentBeginOverlap`
  (params (OverlappedComponent :type "PrimitiveComponent Object Reference") (OtherActor :type "Actor Object Reference") (OtherComp :type "PrimitiveComponent Object Reference") (OtherBodyIndex :type Integer) (bFromSweep :type Boolean) (SweepResult :type "HitResult Structure (by ref)"))
  ;[1 1 1] MainSphere1
  (bind _asbp_pedestrian (cast `/Game/MyContent/BluePrints/Pedestrian/BP_Pedestrian` OtherActor))
  (bind _capsulecomponent (`Character.CapsuleComponent` _asbp_pedestrian))
  (if (== _capsulecomponent OtherComp)
    (`/Engine/EditorBlueprintResources/StandardMacros.IncrementInt` (`self.iCountSphere1-12`)
      (:`  `
        (bind (_returnvalue_x _returnvalue_y) (`KismetMathLibrary.BreakVector` (- (`self.K2_GetActorLocation`) (`SceneComponent.K2_GetComponentLocation` _capsulecomponent))))
        (`KismetArrayLibrary.Array_Append` (`self.ListAxisPoints`) (`|MakeArray` _returnvalue_x _returnvalue_y))))))

(event `self.Sphere1-5.OnComponentBeginOverlap`
  (params (OverlappedComponent :type "PrimitiveComponent Object Reference") (OtherActor :type "Actor Object Reference") (OtherComp :type "PrimitiveComponent Object Reference") (OtherBodyIndex :type Integer) (bFromSweep :type Boolean) (SweepResult :type "HitResult Structure (by ref)"))
  ;[1 1 1] MainSphere1
  (bind _asbp_pedestrian (cast `/Game/MyContent/BluePrints/Pedestrian/BP_Pedestrian` OtherActor))
  (bind _capsulecomponent (`Character.CapsuleComponent` _asbp_pedestrian))
  (if (== _capsulecomponent OtherComp)
    (`/Engine/EditorBlueprintResources/StandardMacros.IncrementInt` (`self.iCountSphere1-5`)
      (:`  `
        (bind (_returnvalue_x _returnvalue_y) (`KismetMathLibrary.BreakVector` (- (`self.K2_GetActorLocation`) (`SceneComponent.K2_GetComponentLocation` _capsulecomponent))))
        (`KismetArrayLibrary.Array_Append` (`self.ListAxisPoints`) (`|MakeArray` _returnvalue_x _returnvalue_y))))))

(event `self.Sphere1-13.OnComponentBeginOverlap`
  (params (OverlappedComponent :type "PrimitiveComponent Object Reference") (OtherActor :type "Actor Object Reference") (OtherComp :type "PrimitiveComponent Object Reference") (OtherBodyIndex :type Integer) (bFromSweep :type Boolean) (SweepResult :type "HitResult Structure (by ref)"))
  ;[1 1 1] MainSphere1
  (bind _asbp_pedestrian (cast `/Game/MyContent/BluePrints/Pedestrian/BP_Pedestrian` OtherActor))
  (bind _capsulecomponent (`Character.CapsuleComponent` _asbp_pedestrian))
  (if (== _capsulecomponent OtherComp)
    (`/Engine/EditorBlueprintResources/StandardMacros.IncrementInt` (`self.iCountSphere1-13`)
      (:`  `
        (bind (_returnvalue_x _returnvalue_y) (`KismetMathLibrary.BreakVector` (- (`self.K2_GetActorLocation`) (`SceneComponent.K2_GetComponentLocation` _capsulecomponent))))
        (`KismetArrayLibrary.Array_Append` (`self.ListAxisPoints`) (`|MakeArray` _returnvalue_x _returnvalue_y))))))

(event `self.Sphere1-6.OnComponentBeginOverlap`
  (params (OverlappedComponent :type "PrimitiveComponent Object Reference") (OtherActor :type "Actor Object Reference") (OtherComp :type "PrimitiveComponent Object Reference") (OtherBodyIndex :type Integer) (bFromSweep :type Boolean) (SweepResult :type "HitResult Structure (by ref)"))
  ;[1 1 1] MainSphere1
  (bind _asbp_pedestrian (cast `/Game/MyContent/BluePrints/Pedestrian/BP_Pedestrian` OtherActor))
  (bind _capsulecomponent (`Character.CapsuleComponent` _asbp_pedestrian))
  (if (== _capsulecomponent OtherComp)
    (`/Engine/EditorBlueprintResources/StandardMacros.IncrementInt` (`self.iCountSphere1-6`)
      (:`  `
        (bind (_returnvalue_x _returnvalue_y) (`KismetMathLibrary.BreakVector` (- (`self.K2_GetActorLocation`) (`SceneComponent.K2_GetComponentLocation` _capsulecomponent))))
        (`KismetArrayLibrary.Array_Append` (`self.ListAxisPoints`) (`|MakeArray` _returnvalue_x _returnvalue_y))))))

(event `self.Sphere1-14.OnComponentBeginOverlap`
  (params (OverlappedComponent :type "PrimitiveComponent Object Reference") (OtherActor :type "Actor Object Reference") (OtherComp :type "PrimitiveComponent Object Reference") (OtherBodyIndex :type Integer) (bFromSweep :type Boolean) (SweepResult :type "HitResult Structure (by ref)"))
  ;[1 1 1] MainSphere1
  (bind _asbp_pedestrian (cast `/Game/MyContent/BluePrints/Pedestrian/BP_Pedestrian` OtherActor))
  (bind _capsulecomponent (`Character.CapsuleComponent` _asbp_pedestrian))
  (if (== _capsulecomponent OtherComp)
    (`/Engine/EditorBlueprintResources/StandardMacros.IncrementInt` (`self.iCountSphere1-14`)
      (:`  `
        (bind (_returnvalue_x _returnvalue_y) (`KismetMathLibrary.BreakVector` (- (`self.K2_GetActorLocation`) (`SceneComponent.K2_GetComponentLocation` _capsulecomponent))))
        (`KismetArrayLibrary.Array_Append` (`self.ListAxisPoints`) (`|MakeArray` _returnvalue_x _returnvalue_y))))))

(event `self.Sphere1-7.OnComponentBeginOverlap`
  (params (OverlappedComponent :type "PrimitiveComponent Object Reference") (OtherActor :type "Actor Object Reference") (OtherComp :type "PrimitiveComponent Object Reference") (OtherBodyIndex :type Integer) (bFromSweep :type Boolean) (SweepResult :type "HitResult Structure (by ref)"))
  ;[1 1 1] MainSphere1
  (bind _asbp_pedestrian (cast `/Game/MyContent/BluePrints/Pedestrian/BP_Pedestrian` OtherActor))
  (bind _capsulecomponent (`Character.CapsuleComponent` _asbp_pedestrian))
  (if (== _capsulecomponent OtherComp)
    (`/Engine/EditorBlueprintResources/StandardMacros.IncrementInt` (`self.iCountSphere1-7`)
      (:`  `
        (bind (_returnvalue_x _returnvalue_y) (`KismetMathLibrary.BreakVector` (- (`self.K2_GetActorLocation`) (`SceneComponent.K2_GetComponentLocation` _capsulecomponent))))
        (`KismetArrayLibrary.Array_Append` (`self.ListAxisPoints`) (`|MakeArray` _returnvalue_x _returnvalue_y))))))

(event `self.Sphere1-15.OnComponentBeginOverlap`
  (params (OverlappedComponent :type "PrimitiveComponent Object Reference") (OtherActor :type "Actor Object Reference") (OtherComp :type "PrimitiveComponent Object Reference") (OtherBodyIndex :type Integer) (bFromSweep :type Boolean) (SweepResult :type "HitResult Structure (by ref)"))
  ;[1 1 1] MainSphere1
  (bind _asbp_pedestrian (cast `/Game/MyContent/BluePrints/Pedestrian/BP_Pedestrian` OtherActor))
  (bind _capsulecomponent (`Character.CapsuleComponent` _asbp_pedestrian))
  (if (== _capsulecomponent OtherComp)
    (`/Engine/EditorBlueprintResources/StandardMacros.IncrementInt` (`self.iCountSphere1-15`)
      (:`  `
        (bind (_returnvalue_x _returnvalue_y) (`KismetMathLibrary.BreakVector` (- (`self.K2_GetActorLocation`) (`SceneComponent.K2_GetComponentLocation` _capsulecomponent))))
        (`KismetArrayLibrary.Array_Append` (`self.ListAxisPoints`) (`|MakeArray` _returnvalue_x _returnvalue_y))))))

(event `self.Sphere1-8.OnComponentBeginOverlap`
  (params (OverlappedComponent :type "PrimitiveComponent Object Reference") (OtherActor :type "Actor Object Reference") (OtherComp :type "PrimitiveComponent Object Reference") (OtherBodyIndex :type Integer) (bFromSweep :type Boolean) (SweepResult :type "HitResult Structure (by ref)"))
  ;[1 1 1] MainSphere1
  (bind _asbp_pedestrian (cast `/Game/MyContent/BluePrints/Pedestrian/BP_Pedestrian` OtherActor))
  (bind _capsulecomponent (`Character.CapsuleComponent` _asbp_pedestrian))
  (if (== _capsulecomponent OtherComp)
    (`/Engine/EditorBlueprintResources/StandardMacros.IncrementInt` (`self.iCountSphere1-8`)
      (:`  `
        (bind (_returnvalue_x _returnvalue_y) (`KismetMathLibrary.BreakVector` (- (`self.K2_GetActorLocation`) (`SceneComponent.K2_GetComponentLocation` _capsulecomponent))))
        (`KismetArrayLibrary.Array_Append` (`self.ListAxisPoints`) (`|MakeArray` _returnvalue_x _returnvalue_y))))))

(event `self.Sphere1-16.OnComponentBeginOverlap`
  (params (OverlappedComponent :type "PrimitiveComponent Object Reference") (OtherActor :type "Actor Object Reference") (OtherComp :type "PrimitiveComponent Object Reference") (OtherBodyIndex :type Integer) (bFromSweep :type Boolean) (SweepResult :type "HitResult Structure (by ref)"))
  ;[1 1 1] MainSphere1
  (bind _asbp_pedestrian (cast `/Game/MyContent/BluePrints/Pedestrian/BP_Pedestrian` OtherActor))
  (bind _capsulecomponent (`Character.CapsuleComponent` _asbp_pedestrian))
  (if (== _capsulecomponent OtherComp)
    (`/Engine/EditorBlueprintResources/StandardMacros.IncrementInt` (`self.iCountSphere1-16`)
      (:`  `
        (bind (_returnvalue_x _returnvalue_y) (`KismetMathLibrary.BreakVector` (- (`self.K2_GetActorLocation`) (`SceneComponent.K2_GetComponentLocation` _capsulecomponent))))
        (`KismetArrayLibrary.Array_Append` (`self.ListAxisPoints`) (`|MakeArray` _returnvalue_x _returnvalue_y))))))

(fn `DrawArrow`
  (`KismetSystemLibrary.DrawDebugArrow` (`self.K2_GetActorLocation`) (`self.vTarget`) 50.0 (struct :`R` 1.0 :`A` 1.0) 0.0 5.0))

(fn `SetTarget`
  (returns (Output_Get :type "Vector Structure"))
  (bind _output_get (set `self.vTarget` (+ (* (`KismetMathLibrary.GetForwardVector` (`self.K2_GetActorRotation`)) (`self.fMoveDistance`)) (`self.K2_GetActorLocation`))))
  (return _output_get))

(fn `UserConstructionScript`)