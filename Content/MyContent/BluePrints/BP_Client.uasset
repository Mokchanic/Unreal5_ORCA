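; BP_Client is a socket client that connects to a configured IP address and port on BeginPlay.
; On connection it sends three hard-coded floats packed into one byte array, prints a success message, or disconnects if the send fails.
; Incoming messages are read as a fixed four-length string and printed, while the disconnect handler is empty.
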(event `self.ReceiveBeginPlay`
  (`self.Connect` (`self.IPAddress`) (`self.Port`) (`|CreateDelegate` :!event `OnDisconnected`) (`|CreateDelegate` :!event `OnConnected`) (`|CreateDelegate` :!event `OnMessageRecived`)))

(fn `OnConnected`
  (params (ConnectionId :type Integer))
  (bind _returnvalue (`self.SendData` ConnectionId (`self.Concat_BytesBytes` (`self.Conv_FloatToBytes` 3.0) (`self.Conv_FloatToBytes` 20.0) (`self.Conv_FloatToBytes` 100.0))))
  (if _returnvalue
    (`KismetSystemLibrary.PrintString` "Success!")
    (else
      (`self.Disconnect` (`local.ConnectionId`)))))

(fn `OnDisconnected`
  (params (ConnectionId :type Integer)))

(fn `OnMessageRecived`
  (params (ConnectionId :type Integer) (Message :type "Array of Byte (by ref)"))
  (bind _returnvalue (`self.Message_ReadString` Message 4))
  (`KismetSystemLibrary.PrintString` _returnvalue)
  (return))

(fn `UserConstructionScript`)